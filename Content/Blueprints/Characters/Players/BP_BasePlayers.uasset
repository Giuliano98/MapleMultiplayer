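; BP_BasePlayers is a base player character that handles side-to-side movement, jumping and the airborne animation trigger.
; The Move Right / Left axis adds movement input along the control rotation's forward vector.
; Jump input only fires when the character is not falling.
; Jumping or walking off a ledge makes the animation instance jump to its Airborne node, in what appears to be a PaperZD setup.
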(event `self.ReceiveBeginPlay`
  (`parent.ReceiveBeginPlay`))

(event `InputAxis|Move Right / Left`
  (params (AxisValue :type "Float (single-precision)"))
  ;[1 1 1] Move Event
  (`self.AddMovementInput` (`KismetMathLibrary.GetForwardVector` (`self.GetControlRotation`)) AxisValue))

(event `InputAction|Jump`
  (params (Key :type "Key Structure"))
  ;[1 1 1] Jump and Falling Events
  (:`Pressed`
    (if (not (`NavMovementComponent.IsFalling` (`self.CharacterMovement`)))
      (`self.Jump`))))

(event `self.OnWalkingOffLedge`
  (params (PreviousFloorImpactNormal :type "Vector Structure (by ref)") (PreviousFloorContactNormal :type "Vector Structure (by ref)") (PreviousLocation :type "Vector Structure (by ref)") (TimeDelta :type "Float (single-precision)"))
  ;[1 1 1] Jump and Falling Events
  (`PaperZDAnimInstance.JumpToNode` (`PaperZDAnimationComponent.AnimInstance` (`self.AnimationComponent`)) "Airborne" "None" :!label _label))

(event `self.OnJumped`
  ;[1 1 1] Jump and Falling Events
  (goto _label))

(fn `UserConstructionScript`
  (`parent.UserConstructionScript`))