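; BP_PlayerBase is a player character Blueprint, named as a base, that handles basic movement and jumping.
; The Move Right / Left axis adds movement input along the control rotation's forward vector rather than its right vector, scaled by the axis value.
; The Jump action calls Jump only when the movement component is not falling.
; BeginPlay and the construction script only call their parent versions.
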(event `self.ReceiveBeginPlay`
  (`parent.ReceiveBeginPlay`))

(event `InputAxis|Move Right / Left`
  (params (AxisValue :type "Float (single-precision)"))
  ;[1 1 1] Movement Event
  (`self.AddMovementInput` (`KismetMathLibrary.GetForwardVector` (`self.GetControlRotation`)) AxisValue))

(event `InputAction|Jump`
  (params (Key :type "Key Structure"))
  ;[1 1 1] Jump Event
  (:`Pressed`
    (if (not (`NavMovementComponent.IsFalling` (`self.CharacterMovement`)))
      (`self.Jump`))))

(fn `UserConstructionScript`
  (`parent.UserConstructionScript`))